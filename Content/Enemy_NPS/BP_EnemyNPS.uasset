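; Enemy NPC character that spots the player, turns and fires a limited supply of fireballs at them.
; View and attack zone overlaps write AIC_EnemyNPS Blackboard flags; first sighting also changes walk speed, and entering attack range stops movement.
; Attack functions toggle the AnimBP flag, spend ammo, clear HaveFireballs when empty, and spawn aimed projectiles.
; Helpers supply a retreat point away from the player and the Way spline, while a widget references its owner.
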(event OnComponentBeginOverlap(ViewZone)
  (params (OverlappedComponent :type Primitive%20Component%20Object%20Reference) (OtherActor :type Actor%20Object%20Reference) (OtherComp :type Primitive%20Component%20Object%20Reference) (OtherBodyIndex :type Integer) (bFromSweep :type Boolean) (SweepResult :type Hit%20Result%20Structure%20%28by%20ref%29))
  ;[1 1 1] Передаем инфу о пересечении зон атаки и видимости
  (AI|Components|Blackboard|SetValueasBool (Variables|/Script/AIModule.AIController|GetBlackboard (Variables|Default|GetSelfController)) (Utilities|Name|MakeLiteralName "InViewRad") true)
  (Utilities|FlowControl|DoOnce false
    (:Completed
      (AI|Components|Blackboard|SetValueasBool (Variables|/Script/AIModule.AIController|GetBlackboard (Variables|Default|GetSelfController)) (Utilities|Name|MakeLiteralName "PlayerWasSeen") true)
      (Variables|/Script/Engine.CharacterMovementComponent|SetMaxWalkSpeed (Variables|Character|GetCharacterMovement) 3e+02))))

(event OnComponentEndOverlap(ViewZone)
  (params (OverlappedComponent :type Primitive%20Component%20Object%20Reference) (OtherActor :type Actor%20Object%20Reference) (OtherComp :type Primitive%20Component%20Object%20Reference) (OtherBodyIndex :type Integer))
  ;[1 1 1] Передаем инфу о пересечении зон атаки и видимости
  (AI|Components|Blackboard|SetValueasBool (Variables|/Script/AIModule.AIController|GetBlackboard (Variables|Default|GetSelfController)) (Utilities|Name|MakeLiteralName "InViewRad") false))

(event OnComponentBeginOverlap(AttackZone)
  (params (OverlappedComponent :type Primitive%20Component%20Object%20Reference) (OtherActor :type Actor%20Object%20Reference) (OtherComp :type Primitive%20Component%20Object%20Reference) (OtherBodyIndex :type Integer) (bFromSweep :type Boolean) (SweepResult :type Hit%20Result%20Structure%20%28by%20ref%29))
  ;[1 1 1] Передаем инфу о пересечении зон атаки и видимости
  (AI|Components|Blackboard|SetValueasBool (Variables|/Script/AIModule.AIController|GetBlackboard (Variables|Default|GetSelfController)) (Utilities|Name|MakeLiteralName "InAttackRad") true)
  (Class|NavMovementComponent|StopActiveMovement (Variables|Character|GetCharacterMovement)))

(event OnComponentEndOverlap(AttackZone)
  (params (OverlappedComponent :type Primitive%20Component%20Object%20Reference) (OtherActor :type Actor%20Object%20Reference) (OtherComp :type Primitive%20Component%20Object%20Reference) (OtherBodyIndex :type Integer))
  ;[1 1 1] Передаем инфу о пересечении зон атаки и видимости
  (AI|Components|Blackboard|SetValueasBool (Variables|/Script/AIModule.AIController|GetBlackboard (Variables|Default|GetSelfController)) (Utilities|Name|MakeLiteralName "InAttackRad") false))

(event EventBeginPlay
  ;[0.108 1 0.3662] Начальные настройки
  (bind _asaic_enemy_nps (Utilities|Casting|CastToAIC_EnemyNPS (AI|GetAIController self)))
  (Variables|Default|SetSelfController _asaic_enemy_nps)
  (bind _asanim_bp_enemy_nps (Utilities|Casting|CastToAnimBP_EnemyNPS (Components|SkeletalMesh|GetAnimInstance (Variables|Character|GetMesh))))
  (Variables|Default|SetSelfAnim _asanim_bp_enemy_nps)
  (bind _returnvalue (Actor|GetActorOfClass "/Game/TopDownBP/Blueprints/TopDownCharacter.TopDownCharacter_C"))
  (Variables|Default|SetPlayer _returnvalue)
  (bind _aswbp_fireballs_count (Utilities|Casting|CastToWBP_FireballsCount (UserInterface|GetWidget (Variables|Default|GetWidget))))
  (Variables|/Game/Enemy_NPS/UI/WBP_FireballsCount.WBP_FireballsCount_C|SetOwner _aswbp_fireballs_count self))

(event EventFunctionStopAttack
  ;[1 1 1] Начинаем/заканчиваем атаку
  (Variables|/Game/Enemy_NPS/Animation/AnimBP_EnemyNPS.AnimBP_EnemyNPS_C|SetIsAttack? (Variables|Default|GetSelfAnim) false))

(event EventFunctionSpawnProjectile
  ;[1 1 1] Спавним фаерболл
  (Game|SpawnActorfromClass "/Game/Enemy_NPS/Projectile/BP_Projectile.BP_Projectile_C" (Math|Transform|MakeTransform (Transformation|GetWorldLocation (Variables|Default|GetProJSpawnPosition)) (Math|Rotator|FindLookatRotation (Transformation|GetWorldLocation (Variables|Default|GetProJSpawnPosition)) (Transformation|GetActorLocation (Variables|Default|GetPlayer)))) "Undefined" 0 (Variables|Default|GetPlayer) 0))

(event EventFunctionStartAttack
  ;[1 1 1] Начинаем/заканчиваем атаку
  (if (> (Variables|Default|GetFireballsCount) 0)
    (Variables|/Game/Enemy_NPS/Animation/AnimBP_EnemyNPS.AnimBP_EnemyNPS_C|SetIsAttack? (Variables|Default|GetSelfAnim) true)
    (Variables|Default|SetFireballsCount (- (Variables|Default|GetFireballsCount) 1))
    (else
      (AI|Components|Blackboard|SetValueasBool (Variables|/Script/AIModule.AIController|GetBlackboard (Variables|Default|GetSelfController)) (Utilities|Name|MakeLiteralName "HaveFireballs") false))))

(event EventFunctionRotatetoAim
  ;[1 1 1] Поворачиваемся к цели
  (Transformation|SetActorRotation (Math|Rotator|MakeRotator 0.0 0.0 (.yaw (Math|Rotator|FindLookatRotation (Transformation|GetActorLocation) (Transformation|GetActorLocation (Variables|Default|GetPlayer))))) true))

(fn ConstructionScript)

(fn FunctionFindLocationAwayfromPlayer
  (bind _returnvalue (Transformation|GetActorLocation))
  (return (+ (* (Math|Vector|GetForwardVector (Math|Rotator|FindLookatRotation (Transformation|GetActorLocation (Variables|Default|GetPlayer)) _returnvalue)) 5e+02) _returnvalue)))

(fn FunctionGetSpline
  (return (Variables|Default|GetWay)))